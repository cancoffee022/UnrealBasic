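; BP_Shotgun is a weapon actor that fires a spread of bullets with each shot.
; Its Fire event checks IsFirable, then spawns several pellets through CreateBullet and sets each projectile's velocity from GetBulletSpeed.
; Spread comes from offsetting a scaled FireDirection by random amounts along the actor's right and up vectors, then normalizing.
; Each volley decrements the remaining bullet count once and updates the last fire time.
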(event `self.Fire`
  (if (`self.IsFirable`)
    (for _ (range 7)
      (bind _returnvalue (`self.CreateBullet`))
      (set `MovementComponent.Velocity` (* (`self.GetBulletSpeed`) (`KismetMathLibrary.Normal` (+ (* (`self.FireDirection`) 200.0) (* (`self.GetActorRightVector`) (`KismetMathLibrary.RandomFloatInRange` -20.0 20.0)) (* (`self.GetActorUpVector`) (`KismetMathLibrary.RandomFloatInRange` -20.0 20.0))))) (`BulletActor.ProjectileMovement` _returnvalue)))
    (`self.DecreaseRemainBullet`)
    (`self.UpdateLastFireTime`)))

(fn `UserConstructionScript`)